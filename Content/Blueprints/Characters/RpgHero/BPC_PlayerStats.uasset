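; Player stats component that tracks health and stamina for BP_ThirdPersonCharacter and mirrors them on its HUD widget.
; BeginPlay waits a tick, caches the owning character and fills the HUD, dividing initial stamina by MaxHealth rather than MaxStamina.
; Decrease functions subtract, update the HUD and return whether the stat is depleted.
; Increase functions add only below a fixed margin under the maximum, without clamping the result.
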(event EventBeginPlay
  (Utilities|FlowControl|DelayUntilNextTick)
  (bind _asbp_third_person_character (Utilities|Casting|CastToBP_ThirdPersonCharacter (Components|GetOwner)))
  (Variables|Default|SetPlayerCharacterBP _asbp_third_person_character)
  (Progress|SetPercent (Variables|/Game/Blueprints/Widgets/WB_HUD.WB_HUD_C|GetHealthBar (Variables|/Game/Blueprints/Characters/RpgHero/BP_ThirdPersonCharacter.BP_ThirdPersonCharacter_C|GetHudWidget (Variables|Default|GetPlayerCharacterBP))) (/ (Variables|Health&Stamina|GetCurrentHealth) (Variables|Health&Stamina|GetMaxHealth)))
  (Rendering|Components|TextRender|SetText (Variables|/Game/Blueprints/Widgets/WB_HUD.WB_HUD_C|GetHealthPercent (Variables|/Game/Blueprints/Characters/RpgHero/BP_ThirdPersonCharacter.BP_ThirdPersonCharacter_C|GetHudWidget (Variables|Default|GetPlayerCharacterBP))) (Utilities|Text|ToText(Float) (Variables|Health&Stamina|GetCurrentHealth) "HalfToEven"))
  (Progress|SetPercent (Variables|/Game/Blueprints/Widgets/WB_HUD.WB_HUD_C|GetStaminaBar (Variables|/Game/Blueprints/Characters/RpgHero/BP_ThirdPersonCharacter.BP_ThirdPersonCharacter_C|GetHudWidget (Variables|Default|GetPlayerCharacterBP))) (/ (Variables|Health&Stamina|GetCurrentStamina) (Variables|Health&Stamina|GetMaxHealth))))

(event EventTick
  (params (DeltaSeconds :type Float%20%28single-precision%29)))

(fn DecreaseHealth
  (params (Damage :type Float%20%28double-precision%29))
  (bind _playercharacterbp (Variables|Default|GetPlayerCharacterBP))
  (bind _hudwidget (Variables|/Game/Blueprints/Characters/RpgHero/BP_ThirdPersonCharacter.BP_ThirdPersonCharacter_C|GetHudWidget _playercharacterbp))
  (if (not (<= (Variables|Health&Stamina|GetCurrentHealth) 0.0))
    (bind _output_get (Variables|Health&Stamina|SetCurrentHealth (- (Variables|Health&Stamina|GetCurrentHealth) Damage)))
    (Progress|SetPercent (Variables|/Game/Blueprints/Widgets/WB_HUD.WB_HUD_C|GetHealthBar _hudwidget) (/ _output_get (Variables|Health&Stamina|GetMaxHealth)))
    (Rendering|Components|TextRender|SetText (Variables|/Game/Blueprints/Widgets/WB_HUD.WB_HUD_C|GetHealthPercent _hudwidget) (Utilities|Text|ToText(Float) (Variables|Health&Stamina|GetCurrentHealth) "HalfToEven"))
    (if (<= (Variables|Health&Stamina|GetCurrentHealth) 0.0)
      (return true)
      (else
        (return false)))))

(fn IncreaseHealth
  (params (HealthIncreament :type Float%20%28double-precision%29))
  (bind _playercharacterbp (Variables|Default|GetPlayerCharacterBP))
  (bind _hudwidget (Variables|/Game/Blueprints/Characters/RpgHero/BP_ThirdPersonCharacter.BP_ThirdPersonCharacter_C|GetHudWidget _playercharacterbp))
  (if (<= (Variables|Health&Stamina|GetCurrentHealth) (- (Variables|Health&Stamina|GetMaxHealth) 1e+01))
    (bind _output_get (Variables|Health&Stamina|SetCurrentHealth (+ (Variables|Health&Stamina|GetCurrentHealth) HealthIncreament)))
    (Progress|SetPercent (Variables|/Game/Blueprints/Widgets/WB_HUD.WB_HUD_C|GetHealthBar _hudwidget) (/ _output_get (Variables|Health&Stamina|GetMaxHealth)))
    (Rendering|Components|TextRender|SetText (Variables|/Game/Blueprints/Widgets/WB_HUD.WB_HUD_C|GetHealthPercent _hudwidget) (Utilities|Text|ToText(Float) (Variables|Health&Stamina|GetCurrentHealth) "HalfToEven"))))

(fn DecreaseStamina
  (params (StaminaDepletion :type Float%20%28double-precision%29))
  (bind _output_get (Variables|Health&Stamina|SetCurrentStamina (- (Variables|Health&Stamina|GetCurrentStamina) StaminaDepletion)))
  (Progress|SetPercent (Variables|/Game/Blueprints/Widgets/WB_HUD.WB_HUD_C|GetStaminaBar (Variables|/Game/Blueprints/Characters/RpgHero/BP_ThirdPersonCharacter.BP_ThirdPersonCharacter_C|GetHudWidget (Variables|Default|GetPlayerCharacterBP))) (/ _output_get (Variables|Health&Stamina|GetMaxStamina)))
  (if (<= (Variables|Health&Stamina|GetCurrentStamina) 0.0)
    (return true)
    (else
      (return false))))

(fn IncreaseStamina
  (params (StaminaIncreament :type Float%20%28double-precision%29))
  (if (<= (Variables|Health&Stamina|GetCurrentStamina) (- (Variables|Health&Stamina|GetMaxStamina) 1.0))
    (bind _output_get (Variables|Health&Stamina|SetCurrentStamina (+ (Variables|Health&Stamina|GetCurrentStamina) StaminaIncreament)))
    (Progress|SetPercent (Variables|/Game/Blueprints/Widgets/WB_HUD.WB_HUD_C|GetStaminaBar (Variables|/Game/Blueprints/Characters/RpgHero/BP_ThirdPersonCharacter.BP_ThirdPersonCharacter_C|GetHudWidget (Variables|Default|GetPlayerCharacterBP))) (/ _output_get (Variables|Health&Stamina|GetMaxStamina)))))